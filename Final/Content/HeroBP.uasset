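; Player hero character with world-axis movement, a visible mouse cursor and click-driven gun fire.
; On BeginPlay it spawns a MousePointBP marker, which each left click moves to the trace hit under the cursor.
; GetGun spawns a GunBP on the mesh's GunSocket, after which pressing and releasing the mouse starts and stops firing.
; The construction script snaps the Left and Right components to the hand sockets.
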(event Custom|GetGun
  (Variables|Default|SetHaveAGun? true)
  (bind _returnvalue (Game|SpawnActorfromClass "/Game/Gun/GunBP.GunBP_C" (Transformation|GetWorldTransform (Variables|Character|GetMesh)) "Undefined" 0 0))
  (bind _output_get (Variables|Default|SetGun _returnvalue))
  (Transformation|AttachComponentToComponent (Variables|/Game/Gun/GunBP.GunBP_C|GetDefaultSceneRoot _output_get) (Variables|Character|GetMesh) "GunSocket" "SnapToTarget" "SnapToTarget" "KeepWorld" true))

(event EventBeginPlay
  (bind _returnvalue (Game|SpawnActorfromClass "/Game/UI/MousePointBP.MousePointBP_C" (Math|Conversions|ToTransform(Vector) (Transformation|GetActorLocation)) "Undefined" 0 0))
  (Variables|Default|SetMouseClickPoint _returnvalue)
  (Variables|/Script/Engine.PlayerController|SetbShowMouseCursor (Game|GetPlayerController 0) true)
  (Variables|Default|SetHaveAGun? false))

(event Collision|EventActorBeginOverlap
  (params (OtherActor :type Actor%20Object%20Reference)))

(event EventTick
  (params (DeltaSeconds :type Float%20%28single-precision%29)))

(event Input|ActionEvents|InputActionLeftMouseClicked
  (params (Key :type Key%20Structure :default "AnyKey"))
  (bind _gun (Variables|Default|GetGun))
  (:Pressed
    (Transformation|SetActorLocation (Variables|Default|GetMouseClickPoint) (.Location (Collision|BreakHitResult (.HitResult (Game|Player|GetHitResultUnderCursorbyChannel (Game|GetPlayerController 0) "TraceTypeQuery1" true)))) false false)
    (if (Variables|Default|GetHaveAGun?)
      (Default|StartFire _gun)))
  (:Released
    (if (Variables|Default|GetHaveAGun?)
      (Default|StopFire _gun))))

(event Input|AxisEvents|InputAxisForward
  (params (AxisValue :type Float%20%28single-precision%29))
  (Pawn|Input|AddMovementInput "1.000000, 0, 0" AxisValue false))

(event Input|AxisEvents|InputAxisLeftRight
  (params (AxisValue :type Float%20%28single-precision%29))
  (Pawn|Input|AddMovementInput "0,1.000000, 0" AxisValue false))

(fn ConstructionScript
  (bind _mesh (Variables|Character|GetMesh))
  (Transformation|AttachComponentToComponent (Variables|Default|GetLeft) _mesh "hand_l" "SnapToTarget" "SnapToTarget" "KeepWorld" true)
  (Transformation|AttachComponentToComponent (Variables|Default|GetRight) _mesh "hand_r" "SnapToTarget" "SnapToTarget" "KeepWorld" true))